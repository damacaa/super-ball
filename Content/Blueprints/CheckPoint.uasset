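; Checkpoint actor that records ordered progress for the player's ball and displays its numeric Id through a text render.
; On overlap it advances the ball's LastCheckpoint only when the previous checkpoint is exactly one below its Id, then prints a message and hides itself.
; It binds to the player ball's reset event on BeginPlay to become visible again, and SetId updates both the Id and the displayed number.
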(event Custom|Reset
  (Rendering|SetActorHiddenInGame false))

(event EventBeginPlay
  (bind _asplayer_ball (Utilities|Casting|CastToPlayerBall (Game|Player|GetPlayerPawn 0)))
  (EventDispatchers|BindEventtoResetEvent _asplayer_ball (delegate Custom|Reset)))

(event Collision|EventActorBeginOverlap
  (params (OtherActor :type Actor%20Object%20Reference))
  (bind _id (Variables|Default|Getid))
  (bind _asplayer_ball (Utilities|Casting|CastToPlayerBall OtherActor))
  (if (== (Variables|/Game/Blueprints/Player/PlayerBall.PlayerBall_C|GetLastCheckpoint _asplayer_ball) (- _id 1))
    (Development|PrintString "Checkpoint")
    (Variables|/Game/Blueprints/Player/PlayerBall.PlayerBall_C|SetLastCheckpoint _asplayer_ball _id)
    (Rendering|SetActorHiddenInGame true)))

(fn ConstructionScript)

(fn SetId
  (params (newId :type Integer))
  (bind _output_get (Variables|Default|Setid newId))
  (Rendering|Components|TextRender|SetText (Variables|Default|GetTextRender) (Utilities|Text|ToText(Integer) _output_get)))