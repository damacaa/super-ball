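; EndGoal is the finish-line actor that declares victory when the PlayerBall overlaps it after reaching the final checkpoint.
; On BeginPlay it counts every TargetPoint in the level as a checkpoint and binds to the player ball's death event, which only prints a taunt.
; On overlap it compares the ball's LastCheckpoint to the last checkpoint index, then prints a message and calls CallVictory on a match.
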(event Custom|PlayerDeathEvent
  (Development|PrintString "You'll never win"))

(event EventBeginPlay
  (bind _asplayer_ball (Utilities|Casting|CastToPlayerBall (Game|Player|GetPlayerPawn 0)))
  (EventDispatchers|BindEventtoPlayerDeath _asplayer_ball (delegate Custom|PlayerDeathEvent))
  (bind _outactors (Actor|GetAllActorsOfClass "/Script/Engine.TargetPoint"))
  (Variables|Default|SetNumberOfCheckpoints (Utilities|Array|Length _outactors)))

(event Collision|EventActorBeginOverlap
  (params (OtherActor :type Actor%20Object%20Reference))
  (bind _asplayer_ball (Utilities|Casting|CastToPlayerBall OtherActor))
  (if (== (Variables|/Game/Blueprints/Player/PlayerBall.PlayerBall_C|GetLastCheckpoint _asplayer_ball) (- (Variables|Default|GetNumberOfCheckpoints) 1))
    (Development|PrintString "Victory")
    (Default|CallVictory)))

(fn ConstructionScript)