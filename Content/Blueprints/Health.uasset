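; Health pickup actor that heals the player ball when it overlaps it.
; After healing, it hides itself and disables collision instead of being destroyed.
; On BeginPlay it binds to the player ball's death event, which makes it visible and collidable again so the pickup respawns whenever the player dies.
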(event Custom|Reset
  (Rendering|SetActorHiddenInGame false)
  (Collision|SetActorEnableCollision true))

(event EventBeginPlay
  (bind _asplayer_ball (Utilities|Casting|CastToPlayerBall (Game|Player|GetPlayerPawn 0)))
  (EventDispatchers|BindEventtoPlayerDeath _asplayer_ball (delegate Custom|Reset)))

(event Collision|EventActorBeginOverlap
  (params (OtherActor :type Actor%20Object%20Reference))
  (bind _asplayer_ball (Utilities|Casting|CastToPlayerBall OtherActor))
  (Default|Heal _asplayer_ball)
  (Rendering|SetActorHiddenInGame true)
  (Collision|SetActorEnableCollision false))

(fn ConstructionScript)