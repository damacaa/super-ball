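; Pendulum Blueprint that swings its Cube component back and forth in pitch.
; BeginPlay waits a random delay of up to a few seconds before playing the Move timeline, so instances can start out of sync.
; Each timeline update sets the Cube's relative pitch, then passes through a fixed Delay that toggles the Loop flag to alternate Play and Reverse.
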(event EventBeginPlay
  (Utilities|FlowControl|Delay (* (Math|Random|RandomFloat) 4.0))
  (bind _move (Timeline|Move Play)
    (:Update
      (Transformation|SetRelativeRotation (Variables|Default|GetCube) (Math|Rotator|MakeRotator 0.0 _move 0.0) false false)
      (Utilities|FlowControl|Delay 4.0)
      (if (Variables|Default|GetLoop)
        (Variables|Default|SetLoop false)
        (Timeline|Move Reverse)
        (else
          (Variables|Default|SetLoop true)
          (Timeline|Move Play))))))

(fn ConstructionScript)