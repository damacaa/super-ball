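; Stage actor that tilts the world around a pivot from two-axis input, relative to the player's view.
; TiltWorld maps X and Y through the control rotation's yaw-only right and forward vectors into local roll and pitch.
; Tick scales roll and pitch by RecoverySpeed and zeroes yaw, presumably easing back to level.
; SetCenter moves the pivot to a given player position and sets World's relative location to its negation.
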(event EventTick
  (params (DeltaSeconds :type Float%20%28single-precision%29))
  (bind _returnvalue (Transformation|GetActorRotation))
  (bind _recoveryspeed (Variables|Default|GetRecoverySpeed))
  (bind (_roll _pitch) (Math|Rotator|BreakRotator _returnvalue))
  (Transformation|SetActorRotation (Math|Rotator|MakeRotator (* _roll _recoveryspeed) (* _pitch _recoveryspeed) 0.0)))

(fn ConstructionScript)

(fn TiltWorld
  (params (x :type Float%20%28double-precision%29) (y :type Float%20%28double-precision%29))
  (bind _returnvalue (Game|Player|GetPlayerPawn 0))
  (bind _tiltspeed (Variables|Default|GetTiltSpeed))
  (bind _tiltspeed_2 (Variables|Default|GetTiltSpeed))
  (bind _returnvalue_2 (Pawn|GetControlRotation _returnvalue :!class /Script/Engine.Pawn))
  (bind _yaw (Math|Rotator|BreakRotator _returnvalue_2))
  (bind _returnvalue_3 (Math|Rotator|MakeRotator 0.0 0.0 _yaw))
  (bind _returnvalue_4 (Math|Vector|GetRightVector _returnvalue_3))
  (bind _returnvalue_5 (Math|Vector|GetForwardVector _returnvalue_3))
  (Transformation|AddActorLocalRotation (Math|Rotator|CombineRotators (Math|Rotator|MakeRotator (* x _tiltspeed_2 (.x _returnvalue_4) -1.0) (* x _tiltspeed_2 (.y _returnvalue_4) -1.0) 0.0) (Math|Rotator|MakeRotator (* y _tiltspeed (.x _returnvalue_5)) (* y _tiltspeed (.y _returnvalue_5)) 0.0)) false false))

(fn SetCenter
  (params (PlayerPosition :type Vector))
  (Transformation|SetActorLocation PlayerPosition false false)
  (Transformation|SetActorRelativeLocation (Variables|Default|GetWorld) (* PlayerPosition -1.0)))